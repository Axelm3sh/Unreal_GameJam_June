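; BP_FloorTile is a self-recycling floor segment for an endless track flown by Player_Missle.
; Construction caches nine spawn-point transforms and randomly adds a blocker child actor at one, with odds set by the game mode's obstacle threshold.
; When the missile overlaps EndTrigger, the tile asks Project_Gamemode to add another tile, then destroys itself after a brief delay.
; GetAttachTransform exposes the AttachPoint world transform, presumably for chaining tiles.
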(event `self.EndTrigger.OnComponentBeginOverlap`
  (params (OverlappedComponent :type "PrimitiveComponent Object Reference") (OtherActor :type "Actor Object Reference") (OtherComp :type "PrimitiveComponent Object Reference") (OtherBodyIndex :type Integer) (bFromSweep :type Boolean) (SweepResult :type "HitResult Structure (by ref)"))
  ;[1 1 1] Floor Tile Creation
  (cast `/Game/Player/Player_Missle` OtherActor)
  (bind _asproject_gamemode (cast `/Game/Blueprints/Project_Gamemode` (`GameplayStatics.GetGameMode`)))
  (`/Game/Blueprints/Project_Gamemode.AddFloorTile` _asproject_gamemode)
  (`KismetSystemLibrary.Delay` 0.075)
  (`self.K2_DestroyActor`))

(fn `GetAttachTransform`
  (returns (AttachTransform :type "Transform Structure"))
  ;[1 1 1] GetAttachTransform Function
  (return (`SceneComponent.K2_GetComponentToWorld` (`self.AttachPoint`))))

(fn `SetSpawnPoints`
  (set `self.SpawnPoints` (`|MakeArray` (`SceneComponent.GetRelativeTransform` (`self.SpawnPointR`)) (`SceneComponent.GetRelativeTransform` (`self.SpawnPointL`)) (`SceneComponent.GetRelativeTransform` (`self.SpawnPoint`)) (`SceneComponent.GetRelativeTransform` (`self.SpawnPointUL`)) (`SceneComponent.GetRelativeTransform` (`self.SpawnPointUC`)) (`SceneComponent.GetRelativeTransform` (`self.SpawnPointUR`)) (`SceneComponent.GetRelativeTransform` (`self.SpawnPointCR`)) (`SceneComponent.GetRelativeTransform` (`self.SpawnPointCC`)) (`SceneComponent.GetRelativeTransform` (`self.SpawnPointCL`)))))

(fn `SpawnBlocker`
  (bind _spawnpoints (`self.SpawnPoints`))
  (bind _asproject_gamemode (cast `/Game/Blueprints/Project_Gamemode` (`GameplayStatics.GetGameMode`)))
  (if (< (`KismetMathLibrary.RandomFloat`) (`/Game/Blueprints/Project_Gamemode.CurrentObstacleThreshhold` _asproject_gamemode))
    (`AddComponent|Child Actor Component_0` :`RelativeTransform` (`KismetArrayLibrary.Array_Get` _spawnpoints (`KismetMathLibrary.RandomIntegerInRange` 0 (`KismetArrayLibrary.Array_LastIndex` _spawnpoints))))))

(fn `UserConstructionScript`
  (`self.SetSpawnPoints`)
  (`self.SpawnBlocker`))