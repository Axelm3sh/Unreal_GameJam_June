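; Wall obstacle block built from two laser pairs, each with start, end and laser components, with horizontal, vertical, spinning and breakable behaviour.
; Horizontal and vertical events each keep one pair by destroying the other.
; Spinner enlarges the actor and sets its RotatingMovement rate.
; Break swaps each surviving part for a destructible component fractured by radius damage from the actor's location, with stronger impulse on lasers and Pair1Start.
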(event `IsHorizontal`
  (`self.ShowHorizontal`))

(event `IsVertical`
  (`self.ShowVertical`))

(event `Spinner`
  (`self.StartSpin`))

(event `self.Break`
  (bind _returnvalue (`self.K2_GetActorLocation`))
  (bind _array (`|MakeArray` (`self.Pair2Laser`) (`self.Pair1Laser`) (`self.Pair1Start`)))
  (bind _array_2 (`|MakeArray` (`self.Pair1End`) (`self.Pair2Start`) (`self.Pair2End`)))
  (for _index (range (+ (`KismetArrayLibrary.Array_Length` _array_2) 1))
    (bind _output (`|GetArrayItem` _array_2 _index))
    (`/Engine/EditorBlueprintResources/StandardMacros.IsValid` _output
      (:`Is Valid`
        (bind _returnvalue_2 (`AddComponent|NODE_AddDestructibleComponent-0` :`RelativeTransform` (`SceneComponent.GetRelativeTransform` _output)))
        (`DestructibleComponent.ApplyRadiusDamage` _returnvalue_2 50.0 _returnvalue 0.0 100.0 true)
        (`ActorComponent.K2_DestroyComponent` _output))))
  (for _index_2 (range (+ (`KismetArrayLibrary.Array_Length` _array) 1))
    (bind _output_2 (`|GetArrayItem` _array _index_2))
    (`/Engine/EditorBlueprintResources/StandardMacros.IsValid` _output_2
      (:`Is Valid`
        (bind _returnvalue_3 (`AddComponent|NODE_AddDestructibleComponent-1` :`RelativeTransform` (`SceneComponent.GetRelativeTransform` _output_2)))
        (`DestructibleComponent.ApplyRadiusDamage` _returnvalue_3 50.0 _returnvalue 0.0 1000.0 true)
        (`ActorComponent.K2_DestroyComponent` _output_2)))))

(fn `ShowHorizontal`
  (`ActorComponent.K2_DestroyComponent` (`self.Pair1End`))
  (`ActorComponent.K2_DestroyComponent` (`self.Pair1Laser`))
  (`ActorComponent.K2_DestroyComponent` (`self.Pair1Start`)))

(fn `ShowVertical`
  (`ActorComponent.K2_DestroyComponent` (`self.Pair2Start`))
  (`ActorComponent.K2_DestroyComponent` (`self.Pair2End`))
  (`ActorComponent.K2_DestroyComponent` (`self.Pair2Laser`)))

(fn `StartSpin`
  (`self.SetActorRelativeScale3D` (1.75 1.75 1.75))
  (set `RotatingMovementComponent.RotationRate` (struct :`Roll` 45.0) (`self.RotatingMovement`)))

(fn `UserConstructionScript`
  (`parent.UserConstructionScript`))