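; BP_HallwayBlock is a hallway obstacle piece built from five wall child actors: left, right, up, down and center.
; Four events pick its shape by destroying unneeded pieces, leaving a center block (pitched 90 degrees for vertical) or an opposing pair around a vertical or horizontal hole.
; Break calls Break on each surviving piece's BP_WallMesh in turn, skipping destroyed components.
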(event `IsCenterHorizontal`
  (`ActorComponent.K2_DestroyComponent` (`self.BlockL`))
  (`ActorComponent.K2_DestroyComponent` (`self.BlockR`))
  (`ActorComponent.K2_DestroyComponent` (`self.BlockD`))
  (`ActorComponent.K2_DestroyComponent` (`self.BlockU`)))

(event `IsCenterVertical`
  (`self.K2_SetActorRelativeRotation` (struct :`Roll` 90.0))
  (`ActorComponent.K2_DestroyComponent` (`self.BlockL`))
  (`ActorComponent.K2_DestroyComponent` (`self.BlockR`))
  (`ActorComponent.K2_DestroyComponent` (`self.BlockD`))
  (`ActorComponent.K2_DestroyComponent` (`self.BlockU`)))

(event `IsVerticalHole`
  (`ActorComponent.K2_DestroyComponent` (`self.BlockC`))
  (`ActorComponent.K2_DestroyComponent` (`self.BlockD`))
  (`ActorComponent.K2_DestroyComponent` (`self.BlockU`)))

(event `IsHorizontalHole`
  (`ActorComponent.K2_DestroyComponent` (`self.BlockC`))
  (`ActorComponent.K2_DestroyComponent` (`self.BlockL`))
  (`ActorComponent.K2_DestroyComponent` (`self.BlockR`)))

(event `self.Break`
  (bind _blockl (`self.BlockL`))
  (bind _blockr (`self.BlockR`))
  (bind _blocku (`self.BlockU`))
  (bind _blockd (`self.BlockD`))
  (bind _blockc (`self.BlockC`))
  (`/Engine/EditorBlueprintResources/StandardMacros.IsValid` _blockl
    (:`Is Valid`
      (bind _asbp_wall_mesh (cast `/Game/Blueprints/BP_WallMesh` (`ChildActorComponent.ChildActor` _blockl)))
      (`/Game/Blueprints/BP_WallMesh.Break` _asbp_wall_mesh))
    (:`Is Not Valid`
      _))
  (`/Engine/EditorBlueprintResources/StandardMacros.IsValid` _blockr
    (:`Is Valid`
      (bind _asbp_wall_mesh_2 (cast `/Game/Blueprints/BP_WallMesh` (`ChildActorComponent.ChildActor` _blockr)))
      (`/Game/Blueprints/BP_WallMesh.Break` _asbp_wall_mesh_2))
    (:`Is Not Valid`
      _))
  (`/Engine/EditorBlueprintResources/StandardMacros.IsValid` _blocku
    (:`Is Valid`
      (bind _asbp_wall_mesh_3 (cast `/Game/Blueprints/BP_WallMesh` (`ChildActorComponent.ChildActor` _blocku)))
      (`/Game/Blueprints/BP_WallMesh.Break` _asbp_wall_mesh_3))
    (:`Is Not Valid`
      _))
  (`/Engine/EditorBlueprintResources/StandardMacros.IsValid` _blockd
    (:`Is Valid`
      (bind _asbp_wall_mesh_4 (cast `/Game/Blueprints/BP_WallMesh` (`ChildActorComponent.ChildActor` _blockd)))
      (`/Game/Blueprints/BP_WallMesh.Break` _asbp_wall_mesh_4))
    (:`Is Not Valid`
      _))
  (`/Engine/EditorBlueprintResources/StandardMacros.IsValid` _blockc
    (:`Is Valid`
      (bind _asbp_wall_mesh_5 (cast `/Game/Blueprints/BP_WallMesh` (`ChildActorComponent.ChildActor` _blockc)))
      (`/Game/Blueprints/BP_WallMesh.Break` _asbp_wall_mesh_5))))

(fn `UserConstructionScript`
  (`parent.UserConstructionScript`))