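; BP_WallMesh is a wall built from nine static mesh pieces that can be shattered through a Break event.
; Break loops over the valid pieces, adds a destructible component at each one's relative transform, then destroys the original mesh.
; Each new destructible immediately receives full radius damage with an impulse, using the piece's relative location, not world location, as the hurt origin.
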(event `Break`
  (bind _array (`|MakeArray` (`self.StaticMesh4`) (`self.StaticMesh1`) (`self.StaticMesh2`) (`self.StaticMesh3`) (`self.StaticMesh`) (`self.StaticMesh5`) (`self.StaticMesh6`) (`self.StaticMesh7`) (`self.StaticMesh8`)))
  (for _index (range (+ (`KismetArrayLibrary.Array_Length` _array) 1))
    (bind _item (`KismetArrayLibrary.Array_Get` _array _index))
    (`/Engine/EditorBlueprintResources/StandardMacros.IsValid` _item
      (:`Is Valid`
        (bind _returnvalue (`SceneComponent.GetRelativeTransform` _item))
        (bind _returnvalue_2 (`AddComponent|Destructible Component_0` :`RelativeTransform` _returnvalue))
        (`DestructibleComponent.ApplyRadiusDamage` _returnvalue_2 50.0 (.location _returnvalue) 0.0 100.0 true)
        (`ActorComponent.K2_DestroyComponent` _item)))))

(fn `UserConstructionScript`)