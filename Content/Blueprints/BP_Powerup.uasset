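; Powerup pickup that spins every tick and is collected when a Player_Missle overlaps its mesh.
; The construction script randomly picks one of three types, swapping in a bottle or sickle mesh for two and keeping the default mesh for the third.
; On overlap it adds a destructible component, using the mesh's transform for bottles, applies radius damage to it, plays a sound and destroys itself.
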(event `self.ReceiveTick`
  (params (DeltaSeconds :type "Float (single-precision)"))
  (`self.K2_AddActorLocalRotation` (struct :`Yaw` 0.75)))

(event `self.PowerupMesh.OnComponentBeginOverlap`
  (params (OverlappedComponent :type "PrimitiveComponent Object Reference") (OtherActor :type "Actor Object Reference") (OtherComp :type "PrimitiveComponent Object Reference") (OtherBodyIndex :type Integer) (bFromSweep :type Boolean) (SweepResult :type "HitResult Structure (by ref)"))
  (bind _returnvalue (`self.K2_GetActorLocation`))
  (cast `/Game/Player/Player_Missle` OtherActor)
  (if (== (`StaticMeshComponent.StaticMesh` (`self.PowerupMesh`)) "/Game/StaticMeshes/Meshes/SM_Bottle.SM_Bottle")
    (bind _returnvalue_2 (`AddComponent|Destructible Component_0` :`RelativeTransform` (`SceneComponent.GetRelativeTransform` (`self.PowerupMesh`))))
    (`DestructibleComponent.ApplyRadiusDamage` _returnvalue_2 50.0 _returnvalue 0.0 100.0 true)
    (else
      (bind _returnvalue_3 (`AddComponent|DestructibleComponent_1`))
      (`DestructibleComponent.ApplyRadiusDamage` _returnvalue_3 50.0 _returnvalue 0.0 100.0 true)))
  (`GameplayStatics.PlaySound2D` "/Game/Audio/Power_UP.Power_UP")
  (`self.K2_DestroyActor`))

(fn `UserConstructionScript`
  (bind _powerupmesh (`self.PowerupMesh`))
  (switch `int` (`KismetMathLibrary.RandomIntegerInRange` 0 2)
    (:`Default`
      (set `self.PowerupType` "NewEnumerator1" :!label _label)
      (`StaticMeshComponent.SetStaticMesh` _powerupmesh "/Game/StaticMeshes/Meshes/SM_Powerup_Sickle.SM_Powerup_Sickle"))
    (:`0`
      (set `self.PowerupType` "NewEnumerator0")
      (`StaticMeshComponent.SetStaticMesh` _powerupmesh "/Game/StaticMeshes/Meshes/SM_Bottle.SM_Bottle"))
    (:`1`
      (goto _label))
    (:`2`
      (set `self.PowerupType` "NewEnumerator2"))))