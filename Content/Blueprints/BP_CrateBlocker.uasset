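; BP_CrateBlocker is a breakable crate obstacle with hanging and standing variants.
; The HangingCrate and StandingCrate events set the matching static mesh and record the variant in IsHanging.
; Break destroys the mesh component, spawns a destructible component in the branch for that variant, and immediately applies full radius damage at the actor's location to shatter it.
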(event `HangingCrate`
  (`StaticMeshComponent.SetStaticMesh` (`self.Crates`) "/Game/StaticMeshes/Meshes/SM_Crates_1.SM_Crates_1")
  (set `self.isHanging` true))

(event `StandingCrate`
  (`StaticMeshComponent.SetStaticMesh` (`self.Crates`) "/Game/StaticMeshes/Meshes/SM_Crates_2.SM_Crates_2")
  (set `self.isHanging` false))

(event `self.Break`
  (bind _returnvalue (`self.K2_GetActorLocation`))
  (`ActorComponent.K2_DestroyComponent` (`self.Crates`))
  (if (`self.isHanging`)
    (bind _returnvalue_2 (`AddComponent|Destructible Component_0`))
    (`DestructibleComponent.ApplyRadiusDamage` _returnvalue_2 100.0 _returnvalue 0.0 100.0 true)
    (else
      (bind _returnvalue_3 (`AddComponent|DestructibleComponent_1`))
      (`DestructibleComponent.ApplyRadiusDamage` _returnvalue_3 100.0 _returnvalue 0.0 100.0 true))))

(fn `UserConstructionScript`
  (`parent.UserConstructionScript`))