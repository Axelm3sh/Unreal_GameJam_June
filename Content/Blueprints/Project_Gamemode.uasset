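; Game mode for an endless runner that builds the track and tracks score and difficulty.
; BeginPlay chains 20 random floor tiles, each spawned at the previous tile's attach transform, with a chance of a curve after a run of straights.
; Each tick adds multiplied points while the player lives and updates the HUD.
; A step counter periodically raises the obstacle threshold, and events set the score multiplier and powerup threshold.
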(event `self.ReceiveBeginPlay`
  (for _ (range 20)
    (`self.AddFloorTile`)))

(event `self.ReceiveTick`
  (params (DeltaSeconds :type "Float (single-precision)"))
  (`self.IncrementPlayerScore`)
  ;[1 1 1] When to ramp up obstacle spawn threshold
  (if (>= (`self.ScoreDifficultyStep`) 2000)
    (set `self.ScoreDifficultyStep` 0)
    (`self.RaiseObstacleThreshold`)))

(event `ChangeScoreMultiplier`
  (params (Multiplier :type "Float (double-precision)"))
  ;[1 1 1] Change score multiplier
  (set `self.PlayerScoreMultiplier` Multiplier))

(event `ChangePowerupThreshold`
  (params (PowerupMultiplier :type "Float (double-precision)"))
  ;[1 1 1] Change Powerup Threshold percentage
  (set `self.PowerupSpawnThreshold` PowerupMultiplier))

(fn `AddFloorCurve`
  (bind _floor_curves (`self.Floor Curves`))
  (bind _returnvalue (`|SpawnActorFromClass` (`KismetArrayLibrary.Array_Get` _floor_curves (`KismetMathLibrary.RandomIntegerInRange` 0 (`KismetArrayLibrary.Array_LastIndex` _floor_curves))) (`self.NextSpawnPoint`) "Undefined" "OverrideRootScale"))
  (bind _asbp_floor_tile (cast `/Game/Blueprints/BP_FloorTile` _returnvalue))
  (bind _attachtransform (`/Game/Blueprints/BP_FloorTile.GetAttachTransform` _asbp_floor_tile))
  (set `self.NextSpawnPoint` _attachtransform)
  (set `self.CurrentStraights` 0))

(fn `AddFloorTile`
  (bind _floortiles (`self.FloorTiles`))
  (if (> (`self.CurrentStraights`) 7)
    (if (< (`KismetMathLibrary.RandomFloat`) 0.25)
      (`self.AddFloorCurve`)
      (else
        (bind _returnvalue (`|SpawnActorFromClass` (`KismetArrayLibrary.Array_Get` _floortiles (`KismetMathLibrary.RandomIntegerInRange` 0 (`KismetArrayLibrary.Array_LastIndex` _floortiles))) (`self.NextSpawnPoint`) "AlwaysSpawn" "OverrideRootScale" :!label _label))
        (bind _asbp_floor_tile (cast `/Game/Blueprints/BP_FloorTile` _returnvalue))
        (bind _attachtransform (`/Game/Blueprints/BP_FloorTile.GetAttachTransform` _asbp_floor_tile))
        (set `self.NextSpawnPoint` _attachtransform)
        (set `self.CurrentStraights` (+ (`self.CurrentStraights`) 1))))
    (else
      (goto _label))))

(fn `IncrementPlayerScore`
  ;[1 1 1] Increment Player points with multiplier
  (if (not (`self.isPlayerDead`))
    (set `self.PlayerScoreTotal` (+ (`self.PlayerScoreTotal`) (`KismetMathLibrary.FTrunc` (* (`self.PlayerScoreMultiplier`) 25.0))))
    ;[1 1 1] Difficulty step increment
    (bind _result (`/Engine/EditorBlueprintResources/StandardMacros.IncrementInt` (`self.ScoreDifficultyStep`))
      (:`  `
        (set `self.ScoreDifficultyStep` _result)
        ;[1 1 1] Display HUD Player score
        (bind _asproject_controller (cast `/Game/Player/Project_Controller` (`GameplayStatics.GetPlayerController` 0)))
        (bind _asplayer_hud (cast `/Game/MainMenu/PlayerHUD` (`/Game/Player/Project_Controller.Player_HUD` _asproject_controller)))
        (`TextBlock.SetText` (`/Game/MainMenu/PlayerHUD.PlayerScore` _asplayer_hud) (`|FormatText` "{pt}pts" (`KismetTextLibrary.Conv_IntToText` (`self.PlayerScoreTotal`))))))))

(fn `RaiseObstacleThreshold`
  (bind _output_get (set `self.CurrentObstacleThreshhold` (+ (`self.CurrentObstacleThreshhold`) (`self.IncrementThreshold`))))
  (`KismetSystemLibrary.PrintString` (`KismetStringLibrary.Conv_DoubleToString` _output_get) true true (struct :`R` 0.430421 :`G` 1.0 :`A` 1.0) 0.0))

(fn `UserConstructionScript`)