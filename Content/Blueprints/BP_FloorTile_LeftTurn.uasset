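; Left-turn floor tile that lets the Player_Missle turn when it overlaps the tile's TurnZone.
; The Construction Script shapes three spline meshes from start and end marker components, taking each end tangent from its end marker's rotation.
; It also randomly reveals, most of the time, one of three decal spots with a material picked from DecalPool.
; BeginPlay and Tick are unused.
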(event `self.TurnZone.OnComponentBeginOverlap`
  (params (OverlappedComponent :type "PrimitiveComponent Object Reference") (OtherActor :type "Actor Object Reference") (OtherComp :type "PrimitiveComponent Object Reference") (OtherBodyIndex :type Integer) (bFromSweep :type Boolean) (SweepResult :type "HitResult Structure (by ref)"))
  (bind _asplayer_missle (cast `/Game/Player/Player_Missle` OtherActor))
  (`/Game/Player/Player_Missle.SetCanTurn` _asplayer_missle true))

(fn `UserConstructionScript`
  (bind _splinemesh01 (`self.SplineMesh01`))
  (bind _splinemesh02 (`self.SplineMesh02`))
  (bind _splinemesh03 (`self.SplineMesh03`))
  (bind _endcurve02 (`self.EndCurve02`))
  (bind _endcurve03 (`self.EndCurve03`))
  (bind _decalspot1 (`self.DecalSpot1`))
  (bind _decalspot2 (`self.DecalSpot2`))
  (bind _decalspot3 (`self.DecalSpot3`))
  (bind _decalpool (`self.DecalPool`))
  (bind _endcurve01 (`self.EndCurve01`))
  (bind _output (`|GetArrayItem` _decalpool (`KismetMathLibrary.RandomInteger` (`KismetArrayLibrary.Array_Length` _decalpool))))
  ;[1 1 1] Shoddy Spline Points
  (`SplineMeshComponent.SetStartPosition` _splinemesh01 (`SceneComponent.RelativeLocation` (`self.StartCurve01`)) true)
  (`SplineMeshComponent.SetEndPosition` _splinemesh01 (`SceneComponent.RelativeLocation` _endcurve01) true)
  (`SplineMeshComponent.SetEndTangent` _splinemesh01 (`KismetMathLibrary.Conv_RotatorToVector` (`SceneComponent.RelativeRotation` _endcurve01)) true)
  (`SplineMeshComponent.SetStartPosition` _splinemesh02 (`SceneComponent.RelativeLocation` (`self.StartCurve02`)) true)
  (`SplineMeshComponent.SetEndPosition` _splinemesh02 (`SceneComponent.RelativeLocation` _endcurve02) true)
  (`SplineMeshComponent.SetEndTangent` _splinemesh02 (`KismetMathLibrary.Conv_RotatorToVector` (`SceneComponent.RelativeRotation` _endcurve02)) true)
  (`SplineMeshComponent.SetStartPosition` _splinemesh03 (`SceneComponent.RelativeLocation` (`self.StartCurve03`)) true)
  (`SplineMeshComponent.SetEndPosition` _splinemesh03 (`SceneComponent.RelativeLocation` _endcurve03) true)
  (`SplineMeshComponent.SetEndTangent` _splinemesh03 (`KismetMathLibrary.Conv_RotatorToVector` (`SceneComponent.RelativeRotation` _endcurve03)) true)
  ;[1 1 1] Random Decal spawn
  (if (<= (`KismetMathLibrary.RandomInteger` 5) 3)
    (switch `int` (`KismetMathLibrary.RandomIntegerInRange` 0 2)
      (:`0`
        (`SceneComponent.SetVisibility` _decalspot1 true false)
        (`DecalComponent.SetDecalMaterial` _decalspot1 _output))
      (:`1`
        (`SceneComponent.SetVisibility` _decalspot2 true false)
        (`DecalComponent.SetDecalMaterial` _decalspot2 _output))
      (:`2`
        (`SceneComponent.SetVisibility` _decalspot3 true false)
        (`DecalComponent.SetDecalMaterial` _decalspot3 _output)))))